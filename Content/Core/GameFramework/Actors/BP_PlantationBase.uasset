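; BP_PlantationBase is a plantation actor that hosts a greenhouse plant grid simulated over game time.
; Each game time update passes the time rate to GreenhouseComponent's simulation.
; When it has a parent actor, its construction script sets the grid origin at a fixed offset from that parent.
; Planting and removal events print optional debug messages; random test seeding of fruit plants is left disconnected.
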(event `self.GreenhouseComponent.OnPlantationCreated`
  ;[0.15 0 0 0.5 36] Добавляем рандомные растеня в плантацию после ее создания
)

(event `self.GameTimeComponent.OnGameTimeUpdated`
  ;[0.15 0 0 0.5 36] Обновляем симуляцию плантации когда обновляется игровое время
  (`GreenhouseComponent.UpdateSimulation` (`self.GreenhouseComponent`) (`GameTimeComponent.GameTimeRate` (`self.GameTimeComponent`))))

(event `self.GreenhouseComponent.OnPlantSeeded`
  (params (PlantData :type "PlantData Object Reference") (IndexCell :type Integer))
  ;[0 0 0 0.5 24] Дебаг информация
  (if (`self.bShowDebug`)
    (`KismetSystemLibrary.PrintString` (`KismetStringLibrary.Concat_StrStr` "- Добавлено растение: " (`KismetTextLibrary.Conv_TextToString` (`PlantData.PlantDisplayName` PlantData)) " / Слот: " (`KismetStringLibrary.Conv_IntToString` IndexCell)) true true (struct :`G` 1.0 :`A` 1.0) 5.0)))

(event `self.GreenhouseComponent.OnPlantationPlantRemoved`
  (params (IndexCell :type Integer))
  ;[0 0 0 0.5 24] Дебаг информация
  (if (`self.bShowDebug`)
    (`KismetSystemLibrary.PrintString` (`KismetStringLibrary.Concat_StrStr` "- Слот очищен: " (`KismetStringLibrary.Conv_IntToString` IndexCell)) true true (struct :`R` 1.0 :`A` 1.0) 5.0)))

(fn `ReceiveTick`
  (params (DeltaSeconds :type "Float (single-precision)")))

(fn `UserConstructionScript`
  (bind _returnvalue (`self.GetParentActor`))
  (`/Engine/EditorBlueprintResources/StandardMacros.IsValid` _returnvalue
    (:`Is Valid`
      (set `GreenhouseComponent.GridOrigin` (+ (`self.K2_GetActorLocation` _returnvalue) (-900.0 -800.0 0.0)) (`self.GreenhouseComponent`)))))