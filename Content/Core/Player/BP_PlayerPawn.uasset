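; Player pawn for a greenhouse game that applies the selected tool, watering can or lamp, to plant cells around the cursor on left click.
; It takes the GreenhouseComponent from a child plantation actor and forwards interface calls to plant, remove, harvest and rebuild plots.
; GetCellsInSphere finds affected cells by testing grid cell centers against an XY radius around the cursor hit.
; Tick shows the brush sphere and prints debug info for cells.
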(event `/Game/Core/Interfaces/BPI_GreenhouseInterface.BPI_Notify_SetTool`
  (params (ToolName :type String))
  (set `self.ToolName` ToolName))

(event `/Game/Core/Interfaces/BPI_GreenhouseInterface.BPI_Notify_Recreate`
  ; Пересоздает грядку
  (`GreenhouseComponent.ClearPlantation` (`self.Greenhouse Component`))
  (`GreenhouseComponent.CreatePlantation` (`self.Greenhouse Component`)))

(event `/Game/Core/Interfaces/BPI_GreenhouseInterface.BPI_Notify_RemoveAllPlants`
  ; Удаляет все посадки из слотов теплици
  (for (_ _array_index) (`GreenhouseComponent.GetPlantCells` (`self.Greenhouse Component`))
    (`GreenhouseComponent.RemovePlantAt` (`self.Greenhouse Component`) _array_index)))

(event `Key|LeftMouseButton`
  (params (Key :type "Key Structure"))
  (bind (_bblockinghit _binitialoverlap _time _distance _location _impactpoint) (`GameplayStatics.BreakHitResult` (`PlayerController.GetHitResultUnderCursorByChannel` (`GameplayStatics.GetPlayerController` 0) "TraceTypeQuery1" true)))
  ; Полив растений/Освещение растений
  (:`Pressed`
    (if _bblockinghit
      (if (not (`KismetStringLibrary.IsEmpty` (`self.ToolName`)))
        (bind _returnvalue (`self.GetCellsInSphere` _impactpoint (`self.Radius`)))
        (for _array_element _returnvalue
          (bind (_foundplant _returnvalue_2) (`GreenhouseComponent.FindPlantCellByCoords` (`self.Greenhouse Component`) _array_element))
          (if _returnvalue_2
            (switch `string` (`self.ToolName`)
              (:`Лейка`
                (bind _returnvalue_3 (`GreenhouseLibrary.GetIndexPlantCell` _foundplant))
                (`GreenhouseComponent.SetResourceValueToPlantCell` (`self.Greenhouse Component`) (struct :`TagName` "Resource.Water") 50.0 _returnvalue_3))
              (:`Лампа`
                (`GreenhouseComponent.SetResourceValueToPlantCell` (`self.Greenhouse Component`) (struct :`TagName` "Resource.Light") 50.0 _returnvalue_3)))))))))

(fn `BPI_Notify_CollectRipePlants`
  (returns (bReturnValue :type Boolean))
  (locals (Arr :type "Array of PlantCell Structure"))
  ; Собирает спелые растения
  (bind _output_get (set `local.Arr` (`GreenhouseComponent.FindPlantsByState` (`self.Greenhouse Component`) "PS_ReadyToHarvest")))
  (for _array_element _output_get
    (`GreenhouseComponent.RemovePlantAt` (`self.Greenhouse Component`) (`GreenhouseComponent.GetPlantCellIndex` (`self.Greenhouse Component`) _array_element)))
  (return true))

(fn `BPI_Notify_DrawDebugPlantCell`
  (params (IndexCell :type Integer) (Duration :type "Float (double-precision)"))
  (returns (bReturnValue :type Boolean))
  (locals (FoundCell :type "PlantCell Structure"))
  (set `self.IndexCell` IndexCell)
  (return true))

(fn `BPI_Notify_PlantSeed`
  (params (PlantData :type "PlantData Object Reference") (IndexCell :type Integer))
  (returns (bReturnValue :type Boolean))
  (`/Engine/EditorBlueprintResources/StandardMacros.IsValid` (`self.Greenhouse Component`)
    (:`Is Valid`
      (bind _returnvalue (`GreenhouseComponent.PlantSeed` (`self.Greenhouse Component`) (`local.PlantData`) (`local.IndexCell`)))
      (return _returnvalue))
    (:`Is Not Valid`
      (return false))))

(fn `BPI_Notify_RemovePlantAt`
  (params (IndexCell :type Integer))
  (returns (bReturnValue :type Boolean))
  (`/Engine/EditorBlueprintResources/StandardMacros.IsValid` (`self.Greenhouse Component`)
    (:`Is Valid`
      (bind _returnvalue (`GreenhouseComponent.RemovePlantAt` (`self.Greenhouse Component`) (`local.IndexCell`)))
      (return _returnvalue))
    (:`Is Not Valid`
      (return false))))

(fn `GetCellsInSphere`
  (params (SphereCenter :type "Vector Structure") (SphereRadius :type "Float (double-precision)"))
  (returns (ReturnValue :type "Array of IntPoint Structure"))
  (locals (BoxMin :type "Vector Structure") (BoxMax :type "Vector Structure") (GridMin :type "IntPoint Structure") (GridMax :type "IntPoint Structure") (CurrentCell :type "IntPoint Structure") (X :type Integer) (Y :type Integer) (CellWorldCenter :type "Vector Structure") (DistanceXY :type "Float (double-precision)") (Arr :type "Array of IntPoint Structure"))
  (`/Engine/EditorBlueprintResources/StandardMacros.IsValid` (`self.Greenhouse Component`)
    (:`Is Valid`
      (`KismetArrayLibrary.Array_Clear` (`local.Arr`))
      ; Находим границы AABB
      (set `local.BoxMin` (- (`local.SphereCenter`) (`KismetMathLibrary.MakeVector` (`local.SphereRadius`) (`local.SphereRadius`))))
      (set `local.BoxMax` (+ (`local.SphereCenter`) (`KismetMathLibrary.MakeVector` (`local.SphereRadius`) (`local.SphereRadius`))))
      ; Преобразуем углы AABB в индексы сетки
      (set `local.GridMin` (`GreenhouseComponent.WorldToGrid` (`self.Greenhouse Component`) (`local.BoxMin`)))
      (set `local.GridMax` (`GreenhouseComponent.WorldToGrid` (`self.Greenhouse Component`) (`local.BoxMax`)))
      ; Перебираем все ячейки в прямоугольнике от GridMin до GridMax
      (for _index (range (`GreenhouseComponent.GridWidth` (`self.Greenhouse Component`)))
        (set `local.X` _index)
        (for _index_2 (range (`GreenhouseComponent.GridHeight` (`self.Greenhouse Component`)))
          (set `local.Y` _index_2)
          (bind _output_get (set `local.CurrentCell` (make `IntPoint` (`local.X`) (`local.Y`))))
          ; Проверяем, что координаты валидны (не выходят за границы сетки)
          (if (`GreenhouseComponent.IsGridCoordsValid` (`self.Greenhouse Component`) _output_get)
            ; Получаем центр текущей ячейки в мировых координатах
            (set `local.CellWorldCenter` (`GreenhouseComponent.GridToWorld` (`self.Greenhouse Component`) (`local.CurrentCell`)))
            ; Вычисляем расстояние от центра сферы до центра ячейки (в плоскости XY)
            (bind _output_get_2 (set `local.DistanceXY` (`KismetMathLibrary.VSize2D` (`KismetMathLibrary.MakeVector2D` (.x (- (`local.CellWorldCenter`) (`local.SphereCenter`))) (.y (- (`local.CellWorldCenter`) (`local.SphereCenter`)))))))
            (if (<= _output_get_2 (`local.SphereRadius`))
              (`KismetArrayLibrary.Array_Add` (`local.Arr`) (`local.CurrentCell`))))))
      (return (`local.Arr`)))))

(fn `ReceiveBeginPlay`
  (bind _asbp_plantation_base (cast `/Game/Core/GameFramework/Actors/BP_PlantationBase` (`ChildActorComponent.ChildActor` (`self.PlantationActor`))))
  (set `self.Greenhouse Component` (`/Game/Core/GameFramework/Actors/BP_PlantationBase.GreenhouseComponent` _asbp_plantation_base)))

(fn `ReceiveTick`
  (params (DeltaSeconds :type "Float (single-precision)"))
  (locals (FoundCell :type "PlantCell Structure"))
  (`self.ShowDebugInfoCell` DeltaSeconds)
  (`self.ShowDebugSphere` DeltaSeconds))

(fn `ShowDebugInfoCell`
  (params (DeltaSeconds :type "Float (double-precision)"))
  (locals (FoundCell :type "PlantCell Structure"))
  (bind ((`Resources` _resources)) (break `PlantCell` (`local.FoundCell`)))
  (bind (_foundplant _returnvalue) (`GreenhouseComponent.FindPlantByIndexCell` (`self.Greenhouse Component`) (`self.IndexCell`)))
  ;[0.15 0 0 0.5 64] Debug
  (if (!= (`self.IndexCell`) -1)
    (`/Engine/EditorBlueprintResources/StandardMacros.IsValid` (`self.Greenhouse Component`)
      (:`Is Valid`
        (if _returnvalue
          (if (`GreenhouseLibrary.IsOccupiedPlantCell` _foundplant)
            (set `local.FoundCell` _foundplant)
            (`|ExecutionSequence`
              (:`then_0`
                (`KismetSystemLibrary.PrintString` (`KismetStringLibrary.Concat_StrStr` "- Состояния слота: " (`|GetEnumeratorNameAsString` (`.State` (break `PlantCell` (`local.FoundCell`))))) true true (struct :`G` 0.66 :`B` 1.0 :`A` 1.0) (`local.DeltaSeconds`)))
              (:`then_1`
                (bind _keys (`BlueprintMapLibrary.Map_Keys` _resources))
                (for _array_element _keys
                  (`KismetSystemLibrary.PrintText` (`|FormatText` "- Уровень {resource}: {value1}" (`BlueprintGameplayTagLibrary.GetTagName` _array_element) (`BlueprintMapLibrary.Map_Find` _resources _array_element)) true true (struct :`G` 0.66 :`B` 1.0 :`A` 1.0) (`local.DeltaSeconds`))))
              (:`then_2`
                (`KismetSystemLibrary.PrintString` (`KismetStringLibrary.Concat_StrStr` "- Прогрессия роста: " (`KismetStringLibrary.Conv_DoubleToString` (`.GrowthProgress` (break `PlantCell` (`local.FoundCell`)))) " / " (`KismetStringLibrary.Conv_DoubleToString` (`PlantData.GrowthStages` (`.Data` (break `PlantCell` (`local.FoundCell`)))))) true true (struct :`G` 0.66 :`B` 1.0 :`A` 1.0) (`local.DeltaSeconds`)))
              (:`then_3`
                (`KismetSystemLibrary.PrintText` (`|FormatText` "======= Растение: {PlantDisplayName}, Индекс {Index} =======" (`PlantData.PlantDisplayName` (`.Data` (break `PlantCell` (`local.FoundCell`)))) (`self.IndexCell`)) true true (struct :`G` 0.66 :`B` 1.0 :`A` 1.0) (`local.DeltaSeconds`))))
            (else
              (`KismetSystemLibrary.PrintString` "В СЛОТЕ НЕТ РАСТЕНИЯ!!!" true true (struct :`R` 1.0 :`A` 1.0) (`local.DeltaSeconds`))))
          (else
            (`KismetSystemLibrary.PrintString` "СЛОТ НЕ ВАЛИДНЫЙ!!!" true true (struct :`R` 1.0 :`A` 1.0) (`local.DeltaSeconds`))))))))

(fn `ShowDebugSphere`
  (params (DeltaSeconds :type "Float (double-precision)"))
  (locals (Color :type "LinearColor Structure" :default (struct :`R` 1.0 :`G` 1.0 :`B` 1.0 :`A` 1.0)))
  (bind (_bblockinghit _binitialoverlap _time _distance _location _impactpoint) (`GameplayStatics.BreakHitResult` (`PlayerController.GetHitResultUnderCursorByChannel` (`GameplayStatics.GetPlayerController` 0) "TraceTypeQuery1" true)))
  (switch `string` (`self.ToolName`)
    (:`Лейка`
      (set `local.Color` (struct :`G` 0.938677 :`B` 1.0 :`A` 1.0)))
    (:`Лампа`
      (set `local.Color` (struct :`R` 0.741619 :`B` 1.0 :`A` 1.0))))
  (if _bblockinghit
    (`KismetSystemLibrary.DrawDebugSphere` _impactpoint (`self.Radius`) 12 (`local.Color`) 0.05 2.0)
    (bind _returnvalue (`self.GetCellsInSphere` _impactpoint (`self.Radius`)))
    (for _array_element _returnvalue
      (`KismetSystemLibrary.PrintString` (`KismetStringLibrary.Concat_StrStr` "Ячейка в радиусе: " (`KismetStringLibrary.Conv_IntToString` (`GreenhouseLibrary.GetIndexPlantCell` (`GreenhouseComponent.FindPlantCellByCoords` (`self.Greenhouse Component`) _array_element)))) true true (struct :`R` 0.40166 :`G` 1.0 :`A` 1.0) (`local.DeltaSeconds`)))))

(fn `UserConstructionScript`)